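; BP_Enemy is a rifle-carrying enemy character that turns to face the player and handles its own death.
; Every tick it sets its yaw from a look-at rotation between its last movement update location and the player.
; Die passes a random death variant to BP_AnimEnemy, destroys the capsule and disables collision on the mesh and rifle.
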(event `self.ReceiveTick`
  (params (DeltaSeconds :type "Float (single-precision)"))
  (bind (_returnvalue_roll _returnvalue_pitch _returnvalue_yaw) (`KismetMathLibrary.BreakRotator` (`KismetMathLibrary.FindLookAtRotation` (`CharacterMovementComponent.GetLastUpdateLocation` (`self.CharacterMovement`)) (`self.K2_GetActorLocation` (`GameplayStatics.GetPlayerCharacter` 0)))))
  (`self.K2_SetActorRotation` (`KismetMathLibrary.MakeRotator` 0.0 0.0 _returnvalue_yaw)))

(fn `Die`
  (bind _asbp_anim_enemy (cast `/Game/BP_Project1/BP_Project1/Enemy/BP_AnimEnemy` (`SkeletalMeshComponent.GetAnimInstance` (`self.Mesh`))))
  (set `/Game/BP_Project1/BP_Project1/Enemy/BP_AnimEnemy.Death` (`KismetMathLibrary.RandomIntegerInRange` 1 3) _asbp_anim_enemy)
  (`ActorComponent.K2_DestroyComponent` (`self.CapsuleComponent`))
  (`PrimitiveComponent.SetCollisionEnabled` (`self.Mesh`) "NoCollision")
  (`PrimitiveComponent.SetCollisionEnabled` (`self.Riffle`) "NoCollision"))

(fn `UserConstructionScript`)